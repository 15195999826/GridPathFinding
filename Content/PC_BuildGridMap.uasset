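; Player controller for the build-grid map editor, handling its keyboard shortcuts.
; BeginPlay sets game-only input and immediately switches it to Game and UI, keeping the cursor visible during capture.
; Ctrl+S asks GM_BuildGridMap to save the edited map, passing IncrementalSave.
; All shortcuts are blocked by CanNotInput, and Ctrl+Z undo and Ctrl+Y redo are placeholders that only print TODO messages.
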(event EventBeginPlay
  (Input|SetInputModeGameOnly self false)
  (Input|SetInputModeGameandUI self 0 "DoNotLock" false false))

(event EventTick
  (params (DeltaSeconds :type Float%20%28single-precision%29)))

(event Input|KeyboardEvents|CtrlY
  (params (Key :type Key%20Structure :default "None"))
  (:Pressed
    (if (not (Variables|Default|GetCanNotInput))
      (Development|PrintString "Todo:重做功能"))))

(event Input|KeyboardEvents|CtrlS
  (params (Key :type Key%20Structure :default "None"))
  (:Pressed
    (if (not (Variables|Default|GetCanNotInput))
      (bind _asgm_build_grid_map (Utilities|Casting|CastToGM_BuildGridMap (Game|GetGameMode)))
      (Class|BuildGridMapGameMode|SaveEditingMapSave _asgm_build_grid_map "IncrementalSave"))))

(event Input|KeyboardEvents|CtrlZ
  (params (Key :type Key%20Structure :default "None"))
  (:Pressed
    (if (not (Variables|Default|GetCanNotInput))
      (Development|PrintString "Todo:撤销功能"))))

(fn ConstructionScript)